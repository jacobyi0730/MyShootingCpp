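; Game mode Blueprint for a shooting game that tracks the score and manages the level and game-over screens.
; InitializeHUDforPlayer puts the game level widget on screen, and AddScorea adds a value to the running score.
; ShowGameOverUIa creates the game-over widget once, then shows the cursor, switches input to UI only and pauses the game.
; BeginPlay and Tick are empty, and leftover input-mode and score-widget nodes are unconnected.
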(event `self.InitializeHUDForPlayer`
  (params (NewPlayer :type "PlayerController Object Reference"))
  (bind _returnvalue (`|CreateWidget` "/Game/UI/WBP_GameLevel.WBP_GameLevel_C"))
  (`UserWidget.AddToViewport` _returnvalue 0))

(event `self.ReceiveBeginPlay`)

(fn `Add Scorea`
  (params (value :type Integer))
  (set `self.score` (+ value (`self.score`))))

(fn `ShowGameOverUIa`
  (bind _returnvalue (`GameplayStatics.GetPlayerController` 0))
  (`/Engine/EditorBlueprintResources/StandardMacros.IsValid` (`self.gameOverUI`)
    (:`Is Not Valid`
      (bind _returnvalue_2 (`|CreateWidget` "/Game/UI/WBP_GameOver.WBP_GameOver_C"))
      (bind _output_get (set `self.gameOverUI` _returnvalue_2))
      (`UserWidget.AddToViewport` _output_get 0)
      (set `PlayerController.bShowMouseCursor` true _returnvalue)
      (`WidgetBlueprintLibrary.SetInputMode_UIOnlyEx` _returnvalue null)
      (`GameplayStatics.SetGamePaused` true))))

(fn `UserConstructionScript`)