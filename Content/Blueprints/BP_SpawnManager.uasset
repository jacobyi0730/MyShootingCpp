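; BP_SpawnManager spawns the enemy wave of a shooting game, then hands over to the boss.
; On BeginPlay it gathers all BP_Spawn actors and starts a looping timer that spawns a BP_Enemy at a random point's arrow transform, stepping to the next index to avoid immediate repeats.
; Once MaxMakeCount is reached, it increments the game mode's GameLevel, clears the timer and calls SetMoveState on BP_Boss.
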(event `self.ReceiveBeginPlay`
  (bind _outactors (`GameplayStatics.GetAllActorsOfClass` "/Game/Blueprints/BP_Spawn.BP_Spawn_C"))
  (set `self.SpawnList` _outactors)
  (bind _returnvalue (`KismetSystemLibrary.K2_SetTimerDelegate` (delegate `MakeEnemy`) 0.5 true 1.0))
  (set `self.timerHandle` _returnvalue))

(event `MakeEnemy`
  (if (< (`self.makeCount`) (`self.maxMakeCount`))
    (bind _output_get (set `self.ChooseIndex` (`KismetMathLibrary.RandomIntegerInRange` 0 (`KismetArrayLibrary.Array_LastIndex` (`self.SpawnList`)))))
    (if (== _output_get (`self.PrevChooseIndex`))
      (set `self.ChooseIndex` (mod (+ (`self.ChooseIndex`) 1) (`KismetArrayLibrary.Array_Length` (`self.SpawnList`)))))
    (bind _transform (`/Game/Blueprints/BP_Spawn.GetArrowTransform` (`|GetArrayItem` (`self.SpawnList`) (`self.ChooseIndex`))))
    (`|SpawnActorFromClass` "/Game/Blueprints/BP_Enemy.BP_Enemy_C" _transform "Undefined" "OverrideRootScale" null null)
    (set `self.PrevChooseIndex` (`self.ChooseIndex`))
    (`/Engine/EditorBlueprintResources/StandardMacros.IncrementInt` (`self.makeCount`))
    (else
      (bind _asbp_shooting_game_mode_base (cast `/Game/Blueprints/BP_ShootingGameModeBase` (`GameplayStatics.GetGameMode`)))
      (`/Engine/EditorBlueprintResources/StandardMacros.IncrementInt` (`/Game/Blueprints/BP_ShootingGameModeBase.gameLevel` _asbp_shooting_game_mode_base)
        (:`  `
          (`KismetSystemLibrary.K2_ClearAndInvalidateTimerHandle` (`self.timerHandle`))
          (bind _returnvalue (`GameplayStatics.GetActorOfClass` "/Game/Blueprints/BP_Boss.BP_Boss_C"))
          (`/Game/Blueprints/BP_Boss.SetMoveState` _returnvalue))))))

(fn `UserConstructionScript`)