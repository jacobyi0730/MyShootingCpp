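; BP_Bullet is a bullet actor that awards score in a shooting game when it overlaps another actor.
; On any overlap it casts the game mode to BP_ShootingGameModeBase and calls AddScore with one point, without filtering or destroying either actor.
; Tick is empty, and leftover logic for moving along the up vector at a set speed is disconnected, so this graph does not move the bullet.
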(event `self.ReceiveActorBeginOverlap`
  (params (OtherActor :type "Actor Object Reference"))
  ;[1 1 1] BP_ShootingGameModeBase의 AddScore함수를 호출하고싶다.
  (bind _asbp_shooting_game_mode_base (cast `/Game/Blueprints/BP_ShootingGameModeBase` (`GameplayStatics.GetGameMode`)))
  (`/Game/Blueprints/BP_ShootingGameModeBase.Add Score` _asbp_shooting_game_mode_base 1))

(event `self.ReceiveTick`
  (params (DeltaSeconds :type "Float (single-precision)")))

(fn `UserConstructionScript`)