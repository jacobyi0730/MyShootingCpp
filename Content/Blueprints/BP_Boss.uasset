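; BP_Boss is a boss actor that moves into position, then fires rotating bullet patterns.
; It starts Idle until SetMoveState is called, then Tick lerps it from its spawn point to MoveTarget at a SpeedRate-based pace.
; On arrival it switches to Attack, where a short Delay in Tick throttles BP_EnemyBullet spawns, each stepped around a full circle by a wrapping index.
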(event `self.ReceiveBeginPlay`
  (set `self.state` "NewEnumerator0")
  (set `self.originLocation` (`self.K2_GetActorLocation`)))

(event `self.ReceiveTick`
  (params (DeltaSeconds :type "Float (single-precision)"))
  (bind _index (`self.index`))
  (switch `/Game/Blueprints/EMyBossState` (`self.state`)
    (:`NewEnumerator1`
      (set `self.moveAlpha` (+ (`self.moveAlpha`) (/ (`GameplayStatics.GetWorldDeltaSeconds`) (`self.speedRate`))))
      (`self.K2_SetActorLocation` (`KismetMathLibrary.VLerp` (`self.originLocation`) (`self.K2_GetActorLocation` (`self.moveTarget`)) (`self.moveAlpha`)))
      (if (>= (`self.moveAlpha`) 1.0)
        (set `self.state` "NewEnumerator2")))
    (:`NewEnumerator2`
      (`KismetSystemLibrary.Delay` 0.05)
      (`|SpawnActorFromClass` "/Game/Blueprints/BP_EnemyBullet.BP_EnemyBullet_C" (`KismetMathLibrary.MakeTransform` (`self.K2_GetActorLocation`) (`KismetMathLibrary.Quat_Rotator` (* (`KismetMathLibrary.Conv_RotatorToQuaternion` (struct :`Pitch` 90.0)) (`KismetMathLibrary.Conv_RotatorToQuaternion` (`KismetMathLibrary.MakeRotator` 0.0 0.0 (`KismetMathLibrary.Conv_IntToDouble` (* (`self.index`) 30))))))) "Undefined" "OverrideRootScale" null null)
      (`/Engine/EditorBlueprintResources/StandardMacros.IncrementInt` _index
        (:`  `
          (if (>= _index 12)
            (set `self.index` 0)))))))

(fn `SetMoveState`
  (set `self.state` "NewEnumerator1"))

(fn `UserConstructionScript`)