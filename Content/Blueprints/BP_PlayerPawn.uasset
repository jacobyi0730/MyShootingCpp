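; BP_PlayerPawn is a player pawn Blueprint with an unconnected draft of input-driven movement.
; The draft builds a normalized direction from horizontal and vertical values along the actor's right and up vectors, then scales it by Speed and delta time to offset the location without sweep.
; Tick and the other events are empty, so this movement never runs in this graph.
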(event `self.ReceiveTick`
  (params (DeltaSeconds :type "Float (single-precision)"))
  ;[1 1 1] 사용자의 입력에따라 방향을 만들고
)

(fn `UserConstructionScript`)